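; Player camera pawn that the player pans along the world Y axis by dragging with the left mouse button.
; A gate opened while the button is held runs DragCamera on Tick, offsetting Y by axis input within clamped bounds at fixed height.
; IsObserving disables input and dragging.
; A ReturnToBaseCamera flag, polled each Tick, clears observing, removes all widgets and blends the view back to this player's pawn.
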(event `self.ReceiveTick`
  (params (DeltaSeconds :type "Float (single-precision)"))
  (bind _returnvalue (`GameplayStatics.GetPlayerController` 0))
  (`|ExecutionSequence`
    (:`then_0`
      (if (`self.IsObserving`)
        (`self.DisableInput` _returnvalue)
        (else
          (`self.EnableInput` _returnvalue)
          (`/Engine/EditorBlueprintResources/StandardMacros.Gate` true :!label _label
            (:`Exit`
              (`self.DragCamera`))))))
    (:`then_1`
      (if (`self.Return to Base Camera`)
        (set `self.IsObserving` false)
        (`self.EnableInput` (`GameplayStatics.GetPlayerController` 0))
        (`WidgetLayoutLibrary.RemoveAllWidgets`)
        (`PlayerController.SetViewTargetWithBlend` (`GameplayStatics.GetPlayerController` 0) (`GameplayStatics.GetPlayerPawn` 0) 0.5 "VTBlend_Cubic" 0.0 false)
        (set `self.Return to Base Camera` false)))))

(event `Key|LeftMouseButton`
  (params (Key :type "Key Structure"))
  (:`Pressed`
    (goto _label :!via `Open`))
  (:`Released`
    (goto _label :!via `Close`)))

(fn `DragCamera`
  (bind _camera (`self.Camera`))
  (bind (_returnvalue_x _returnvalue_y) (`KismetMathLibrary.BreakVector` (`SceneComponent.K2_GetComponentLocation` _camera)))
  (bind _returnvalue (* (`self.GetInputAxisKeyValue`) -10.0))
  (if (not (`self.IsObserving`))
    (`SceneComponent.K2_SetWorldLocation` _camera (`KismetMathLibrary.MakeVector` 0.0 (`KismetMathLibrary.FClamp` (+ _returnvalue_y _returnvalue) -1000.0 1000.0) 190.0) false false)
    (`KismetSystemLibrary.PrintString` (`KismetStringLibrary.Conv_DoubleToString` _returnvalue))))

(fn `UserConstructionScript`)